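; BP_TestPlayer is a test player Blueprint for toggling a replicated attack flag over the network.
; Pressing E flips DoAttack on the custom player state, directly with authority or through the RPCServer event on a remote client, and prints the new value.
; The OnRep functions for TestChange and DoAttack, like the construction script, are empty.
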(event Custom|RPC%20Server
  (bind _customplayerstate (Variables|Default|GetCustomPlayerState))
  (bind _output_get (Variables|/Script/SteamMultiplay.CustomPlayerState|SetbDoAttack _customplayerstate (not (Variables|/Script/SteamMultiplay.CustomPlayerState|GetbDoAttack _customplayerstate))))
  (Development|PrintString (Utilities|String|ToString(Boolean) _output_get)))

(event Input|KeyboardEvents|E
  (params (Key :type Key%20Structure :default "None"))
  (bind _customplayerstate (Variables|Default|GetCustomPlayerState))
  (:Pressed
    (Development|PrintString "burron pressed")
    (Networking|SwitchHasAuthority
      (:Authority
        (bind _output_get (Variables|/Script/SteamMultiplay.CustomPlayerState|SetbDoAttack _customplayerstate (not (Variables|/Script/SteamMultiplay.CustomPlayerState|GetbDoAttack _customplayerstate))))
        (Development|PrintString (Utilities|String|ToString(Boolean) _output_get)))
      (:Remote
        (CallFunction|RPCServer self)))))

(fn ConstructionScript)

(fn OnRepTestChange)

(fn OnRepDoAttack)